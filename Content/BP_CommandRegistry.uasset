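; Command registry for an in-game debug console, providing built-in commands for console output, engine control, map loading, quitting and system checks.
; BroadcastCommand stores the raw text and arguments, lowercases the command word, then invokes the same-named function or event through a near-zero SetTimerByFunctionName.
; Each handler reads its arguments from that stored state, with some forwarding to ExecuteConsoleCommand, and reports through DebugConsole or LogToConsole.
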(event Custom|exit
  (bind _debugconsole (Variables|Default|GetDebugConsole))
  (Default|ClearOutput _debugconsole)
  (Default|SendtoLog _debugconsole "NewEnumerator14" "Exiting game! Bye bye...")
  (Utilities|FlowControl|Delay 2.0)
  (Game|QuitGame 0 "Quit" true))

(event Collision|EventActorBeginOverlap
  (params (OtherActor :type Actor%20Object%20Reference)))

(event EventTick
  (params (DeltaSeconds :type Float%20%28single-precision%29)))

(event EventBeginPlay)

(event EventBroadcastCommand
  (params (command_text :type String))
  (Variables|Default|SetRawCommand command_text)
  (bind _output_get (Variables|Default|SetCommand%20Text command_text))
  (Variables|Default|SetCommandArgs (Utilities|String|ParseIntoArray command_text " "))
  (if (Utilities|String|Contains _output_get " ")
    (Variables|Default|SetCommand%20Text (Utilities|String|ToLower (.LeftS (Utilities|String|Split _output_get " ")))))
  (Development|PrintString self (Variables|Default|GetCommand%20Text) false false)
  (CallFunction|LogtoConsole "NewEnumerator21" (Variables|Default|GetRawCommand))
  (Utilities|Time|SetTimerbyFunctionName 0 (Variables|Default|GetCommand%20Text) 0.0001))

(fn ConstructionScript)

(fn Engine
  (Default|SendtoLog (Variables|Default|GetDebugConsole) "NewEnumerator15" (Utilities|String|Append "Engine version: " (Development|GetEngineVersion))))

(fn Res
  (Development|ExecuteConsoleCommand (Utilities|String|Append "r.ScreenPercentage " (Utilities|Array|Get(acopy) (Variables|Default|GetCommandArgs) 1)) 0))

(fn Exec
  (bind _rawcommand (Variables|Default|GetRawCommand))
  (bind _rights (Utilities|String|Split _rawcommand " "))
  (Development|ExecuteConsoleCommand _rights 0)
  (Default|SendtoLog (Variables|Default|GetDebugConsole) "NewEnumerator15" (Utilities|String|Append "Command has been sent to engine: " _rights "[#S007]")))

(fn Platform
  (Default|SendtoLog (Variables|Default|GetDebugConsole) "NewEnumerator15" (Utilities|String|Append "Current platform: " (Game|GetPlatformName))))

(fn Open
  (bind _rawcommand (Variables|Default|GetRawCommand))
  (Development|ExecuteConsoleCommand _rawcommand 0)
  (Default|SendtoLog (Variables|Default|GetDebugConsole) "NewEnumerator15" (Utilities|String|Append "Opening map/server: " (.RightS (Utilities|String|Split _rawcommand " ")) "[#S007]")))

(fn Clear
  (bind _debugconsole (Variables|Default|GetDebugConsole))
  (Default|ClearOutput _debugconsole)
  (Default|SendtoLog _debugconsole "NewEnumerator15" "Cleared console output!"))

(fn Help
  (CallFunction|LogtoConsole "NewEnumerator15" (Utilities|String|Append "List of available commands:

DSHConsoleCommands
clear - clears console output
exec <command> - executes console command
res <scale> - set screen percentage to desired value
exit - Exits a game!
engine - prints engine version and build number
platform - prints platform name" "

" (Variables|/DSHDebugConsole/Blueprints/PDA_ConsoleConfig.PDA_ConsoleConfig_C|GetConsoleHELP (Variables|/DSHDebugConsole/W_DebugConsole.W_DebugConsole_C|GetConsoleConfig (Variables|Default|GetDebugConsole))))))

(fn Checkwine
  (Default|SendtoLog (Variables|Default|GetDebugConsole) "NewEnumerator15" (Utilities|String|Append "IsRunningUnderWine: " (Utilities|String|ToString(Boolean) (Class|IsWineLibrary|IsRunningUnderWine)))))

(fn Checkproc
  (bind _rawcommand (Variables|Default|GetRawCommand))
  (bind _rights (Utilities|String|Split _rawcommand " "))
  (bind _returnvalue (Class|CheckProcessLibrary|IsProcessRunning _rights))
  (Default|SendtoLog (Variables|Default|GetDebugConsole) "NewEnumerator15" (Utilities|String|ToString(Text) (Utilities|Text|FormatText "Is process {process} running: {value}" _rights _returnvalue))))